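; BP_AICharacter is an AI-controlled character that wanders at random, carries a weapon and takes damage.
; On BeginPlay it starts the movement loop, spawns a BP_Weapon attached to its Scene component and initializes health.
; MoveNpc sends it to random reachable nearby points, calling itself again after a pause on success or a brief retry delay on failure.
; AnyDamage reduces Health, clamping it at zero and setting IsDeath when damage exceeds the remaining health.
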(event `self.ReceiveBeginPlay`
  (`self.MoveNpc`)
  (bind _returnvalue (`|SpawnActorFromClass` "/Game/Blueprints/BP_Weapon.BP_Weapon_C" (`KismetMathLibrary.MakeTransform` (0.0 0.0 0.0)) "Undefined" "OverrideRootScale" null null))
  (bind _output_get (set `self.weapon` _returnvalue))
  (`self.K2_AttachToComponent` _output_get (`self.Scene`) "None" "KeepRelative" "KeepRelative" "KeepRelative" true)
  (bind _output_get_2 (set `self.DefaultHealth` 100.0))
  (set `self.Health` _output_get_2)
  (set `self.is_death` false))

(event `MoveNpc`
  (bind _output_get (set `self.Random Location` (`NavigationSystemV1.K2_GetRandomReachablePointInRadius` (`self.K2_GetActorLocation`) 1000.0 null null)))
  (`|AIMoveTo` self _output_get null
    (:`OnSuccess`
      (`KismetSystemLibrary.Delay` 4.0)
      (`self.MoveNpc`))
    (:`OnFail`
      (`KismetSystemLibrary.Delay` 0.1)
      (`self.MoveNpc`))))

(event `self.ReceiveAnyDamage`
  (params (Damage :type "Float (single-precision)") (DamageType :type "DamageType Object Reference") (InstigatedBy :type "Controller Object Reference") (DamageCauser :type "Actor Object Reference"))
  (bind _returnvalue (- (`self.Health`) Damage))
  (if (< _returnvalue 0.0)
    (set `self.Health` 0.0)
    (set `self.is_death` true)
    (else
      (set `self.Health` _returnvalue))))

(fn `UserConstructionScript`)