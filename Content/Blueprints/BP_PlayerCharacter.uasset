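; Player character Blueprint that sets up the player's HUD and weapon and tracks whether the character is dead.
; On BeginPlay it adds a widget for player controller 0 to the viewport, spawns a weapon attached to its Scene component, and pushes the health ratio to the widget.
; Tick sets IsDead by polling current health, while GetWeapon exposes the spawned weapon.
; The widget's RepNotify is empty.
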(event `self.ReceiveBeginPlay`
  (bind _returnvalue (`|CreateWidget` "/Game/Blueprints/Bp_Widget.Bp_Widget_C" (`GameplayStatics.GetPlayerControllerFromID` 0)))
  (bind _output_get (set `self.widget` _returnvalue))
  (`UserWidget.AddToViewport` _output_get 0)
  (bind _returnvalue_2 (`|SpawnActorFromClass` "/Game/Blueprints/BP_Weapon.BP_Weapon_C" (`KismetMathLibrary.MakeTransform` (0.0 0.0 0.0)) "Undefined" "OverrideRootScale" null null))
  (bind _output_get_2 (set `self.weapon` _returnvalue_2))
  (`self.K2_AttachToComponent` _output_get_2 (`self.Scene`) "None" "KeepRelative" "KeepRelative" "KeepRelative" true)
  (`/Game/Blueprints/Bp_Widget.change_health` (`self.widget`) (/ (`self.GetCurrentHealth`) (`self.GetMaxHealth`))))

(event `self.ReceiveTick`
  (params (DeltaSeconds :type "Float (single-precision)"))
  (set `self.is_dead` (<= (`self.GetCurrentHealth`) 0.0)))

(fn `Get_Weapon`
  (returns (ReturnValue :type "Actor Object Reference"))
  (return (`self.weapon`)))

(fn `OnRep_widget`)

(fn `UserConstructionScript`)